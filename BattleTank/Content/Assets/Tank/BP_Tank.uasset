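; Player-controllable tank Blueprint that wires input to aiming, movement and firing.
; On BeginPlay it hands the barrel and turret to TankAiming, and the left and right tracks to TankMovement.
; Move and turn axes pass intents to TankMovement, and Fire calls TankAiming.
; Aim axes split rotation, with yaw on AzimuthGimbal and pitch on SpringArm, applying raw axis values as local rotation deltas.
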(event EventBeginPlay
  (Class|TankAimingComponent|InitialiseAimingComponent (Variables|Default|GetTankAiming) (Variables|Default|GetBarrel) (Variables|Default|GetTurret))
  (Class|TankMovementComponent|InitialiseMovementComponent (Variables|Default|GetTankMovement) (Variables|Default|GetLeft%20Track) (Variables|Default|GetRight%20Track)))

(event Input|ActionEvents|InputActionFire
  (params (Key :type Key%20Structure))
  ;[1 1 1] Balistics Input binding
  (:Pressed
    (Class|TankAimingComponent|Fire (Variables|Default|GetTankAiming))))

(event Input|AxisEvents|InputAxisAimAzimuth
  (params (AxisValue :type Float%20%28single-precision%29))
  ;[1 1 1] Balistics Input binding
  (Transformation|AddLocalRotation (Variables|Default|GetAzimuth%20Gimbal) (Math|Rotator|MakeRotator 0.0 0.0 AxisValue) false false))

(event Input|AxisEvents|InputAxisAimElevation
  (params (AxisValue :type Float%20%28single-precision%29))
  ;[1 1 1] Balistics Input binding
  (Transformation|AddLocalRotation (Variables|Default|GetSpringArm) (Math|Rotator|MakeRotator 0.0 AxisValue 0.0) false false))

(event Input|AxisEvents|InputAxisTurnright
  (params (AxisValue :type Float%20%28single-precision%29))
  ;[1 1 1] Movement Input binding
  (Class|TankMovementComponent|IntendTurnRight (Variables|Default|GetTankMovement) AxisValue))

(event Input|AxisEvents|InputAxisMoveforward
  (params (AxisValue :type Float%20%28single-precision%29))
  ;[1 1 1] Movement Input binding
  (Class|TankMovementComponent|IntendMoveForward (Variables|Default|GetTankMovement) AxisValue))

(fn ConstructionScript)